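; BP_Bomb is a lobbed bomb projectile that launches toward the player and explodes.
; On BeginPlay it randomizes its spin and uses a suggested toss velocity to arc at the player's current position, with debug drawing enabled.
; Hitting a BPI_Interact actor sends KillplayerMessage and detonates it; otherwise it detonates after a timed delay.
; Explode fires a radial impulse, spawns a tinted Niagara poof and destroys the bomb.
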(event OnComponentHit(Sphere)
  (params (HitComponent :type Primitive%20Component%20Object%20Reference) (OtherActor :type Actor%20Object%20Reference) (OtherComp :type Primitive%20Component%20Object%20Reference) (NormalImpulse :type Vector :default "0, 0, 0") (Hit :type Hit%20Result%20Structure%20%28by%20ref%29))
  (if (Utilities|DoesObjectImplementInterface OtherActor "/Game/CORE/Blueprints/BPI_Interact.BPI_Interact_C")
    (Class|BPIInteract|Killplayer(Message) OtherActor)
    (CallFunction|Explode)))

(event EventBeginPlay
  (Variables|/Script/Engine.RotatingMovementComponent|SetRotationRate (Variables|Default|GetRotatingMovement) (Math|Random|RandomRotator true))
  (bind _tossvelocity (Class|GameplayStatics|BlueprintSuggestProjectileVelocity (Transformation|GetActorLocation) (Transformation|GetActorLocation (Game|Player|GetPlayerPawn 0)) (Variables|/Script/Engine.ProjectileMovementComponent|GetInitialSpeed (Variables|Default|GetProjectileMovement)) 0.0 "DoNotTrace" 0.0 false true true))
  (Variables|/Script/Engine.MovementComponent|SetVelocity (Variables|Default|GetProjectileMovement) _tossvelocity)
  (Utilities|FlowControl|Delay 4.0)
  (CallFunction|Explode))

(fn ConstructionScript)

(fn Explode
  (Class|RadialForceComponent|FireImpulse (Variables|Default|GetRadialForce))
  (bind _returnvalue (Niagara|SpawnSystematLocation "/Game/CORE/Niagara/NS_Poof.NS_Poof" (Transformation|GetActorLocation)))
  (Effects|Components|ParticleSystem|SetColorParameter _returnvalue "Maximum_Color" "(R=1.000000,G=0.008260,B=0.000000,A=1.000000)")
  (Effects|Components|ParticleSystem|SetColorParameter _returnvalue "Minimum_Color" "(R=1.000000,G=0.691716,B=0.000000,A=1.000000)")
  (Actor|DestroyActor))