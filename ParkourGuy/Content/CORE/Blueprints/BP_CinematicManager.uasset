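; BP_CinematicManager plays the level's intro and outro level sequences and locks player input while they run.
; The intro starts on BeginPlay, and the IA_Skip input stops it and restores controls.
; ToggleControls disables the player character's input, waits for the sequence's duration with a Delay, then re-enables it.
; The outro uses the same lock, then opens L_MainMenu once the wait ends.
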(event Custom|PlayIntro
  (bind _intro (Variables|Default|GetIntro)
    (:then
      (Sequencer|Player|Play (Variables|/Script/LevelSequence.LevelSequenceActor|GetSequencePlayer _intro) :!class /Script/MovieScene.MovieSceneSequencePlayer)
      (Utilities|ToggleControls (Class|TimeManagementBlueprintLibrary|ToSeconds(QualifiedFrameTime) (Media|MediaPlayer|GetDuration (Variables|/Script/LevelSequence.LevelSequenceActor|GetSequencePlayer (Variables|Default|GetIntro))))))
    (:else
      (Development|PrintString "Intro Not Valid" true true "(R=1.000000,G=0.049519,B=0.000000,A=1.000000)"))))

(event Custom|SkipIntro
  (Sequencer|Player|Stop (Variables|/Script/LevelSequence.LevelSequenceActor|GetSequencePlayer (Variables|Default|GetIntro)) :!class /Script/MovieScene.MovieSceneSequencePlayer)
  (Utilities|ToggleControls 0.0))

(event Custom|PlayOutro
  (bind _outro (Variables|Default|GetOutro)
    (:then
      (Sequencer|Player|Play (Variables|/Script/LevelSequence.LevelSequenceActor|GetSequencePlayer _outro) :!class /Script/MovieScene.MovieSceneSequencePlayer)
      (Utilities|ToggleControls (Class|TimeManagementBlueprintLibrary|ToSeconds(QualifiedFrameTime) (Media|MediaPlayer|GetDuration (Variables|/Script/LevelSequence.LevelSequenceActor|GetSequencePlayer (Variables|Default|GetOutro)))))
      (Game|OpenLevel(byObjectReference) "/Game/CORE/L_MainMenu.L_MainMenu"))
    (:else)))

(event Input|EnhancedActionEvents|EnhancedInputActionIA_Skip
  (params (ActionValue :type Boolean) (ElapsedSeconds :type Float%20%28double-precision%29) (TriggeredSeconds :type Float%20%28double-precision%29) (InputAction :type Input%20Action%20Object%20Reference :default "/Game/ThirdPerson/Input/Actions/IA_Skip.IA_Skip"))
  (:Started
    (CallFunction|SkipIntro)))

(event EventBeginPlay
  (CallFunction|PlayIntro))

(fn ConstructionScript)