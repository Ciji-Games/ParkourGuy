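; BP_CustomDecal is a decal actor whose color, texture and size parameters are driven by its own variables.
; The construction script creates a dynamic instance of the decal component's material, passes in Color, Texture and Size as SizeU and SizeV, then assigns it back to the decal.
; All setup happens in the construction script, with no active event graph logic.
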(event EventBeginPlay)

(event Collision|EventActorBeginOverlap
  (params (OtherActor :type Actor%20Object%20Reference)))

(event EventTick
  (params (DeltaSeconds :type Float%20%28single-precision%29)))

(fn ConstructionScript
  (bind _returnvalue (Rendering|Material|CreateDynamicMaterialInstance (Class|DecalComponent|GetDecalMaterial (Variables|Default|GetDecal)) "None" "None" :!class /Script/Engine.KismetMaterialLibrary))
  (Variables|Default|SetDynMat _returnvalue)
  (Rendering|Material|SetVectorParameterValue (Variables|Default|GetDynMat) "Color" (Variables|Default|GetColor) :!class /Script/Engine.MaterialInstanceDynamic)
  (Rendering|Material|SetTextureParameterValue (Variables|Default|GetDynMat) "Texture" (Variables|Default|GetTexture))
  (Rendering|Material|SetScalarParameterValue (Variables|Default|GetDynMat) "SizeU" (.x (Variables|Default|GetSize)) :!class /Script/Engine.MaterialInstanceDynamic)
  (Rendering|Material|SetScalarParameterValue (Variables|Default|GetDynMat) "SizeV" (.y (Variables|Default|GetSize)) :!class /Script/Engine.MaterialInstanceDynamic)
  (Rendering|Components|Decal|SetDecalMaterial (Variables|Default|GetDecal) (Variables|Default|GetDynMat)))