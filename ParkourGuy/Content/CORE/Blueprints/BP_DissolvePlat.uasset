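; BP_DissolvePlat is a wooden platform that moves along a spline and temporarily disappears after the player steps on it.
; A Timeline with configurable start position, play rate and curve drives the floor mesh's location along the spline.
; Player overlap with the Box activates a Niagara effect at once and starts parallel delays that hide and disable collision, then restore both a few seconds later.
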(event OnComponentBeginOverlap(Box)
  (params (OverlappedComponent :type Primitive%20Component%20Object%20Reference) (OtherActor :type Actor%20Object%20Reference) (OtherComp :type Primitive%20Component%20Object%20Reference) (OtherBodyIndex :type Integer) (bFromSweep :type Boolean) (SweepResult :type Hit%20Result%20Structure%20%28by%20ref%29))
  (if (== OtherActor (Game|Player|GetPlayerPawn 0))
    (Utilities|FlowControl|Sequence
      (:then_0
        (Utilities|FlowControl|Delay 4.0)
        (Development|SetHiddeninGame (Variables|Default|Getfloor_wood_2x2) true false)
        (Collision|SetCollisionEnabled (Variables|Default|GetBox) "NoCollision"))
      (:then_1
        (Utilities|FlowControl|Delay 8.0)
        (Development|SetHiddeninGame (Variables|Default|Getfloor_wood_2x2) false false)
        (Collision|SetCollisionEnabled (Variables|Default|GetBox) "QueryAndPhysics"))
      (:then_2
        (Components|Activation|Activate (Variables|Default|GetNiagara) true)))))

(event EventBeginPlay
  (Components|Timeline|SetNewTime (Variables|Default|GetTimeline) (Math|Float|MapRangeClamped (Variables|Default|GetStartPos) 0.0 1.0 0.0 (Components|Timeline|GetTimelineLength (Variables|Default|GetTimeline))))
  (Components|Timeline|SetPlayRate (Variables|Default|GetTimeline) (Variables|Default|GetNewRate))
  (Class|TimelineComponent|SetFloatCurve (Variables|Default|GetTimeline) (Variables|Default|GetNew%20Float%20Curve) "Progress")
  (bind _progress (Timeline|Timeline Play)
    (:Update
      (Transformation|SetRelativeLocation (Variables|Default|Getfloor_wood_2x2) (Spline|GetLocationatTime (Variables|Default|GetSpline) _progress "Local" false) false false))))

(fn ConstructionScript)