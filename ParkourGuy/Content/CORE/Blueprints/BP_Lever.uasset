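; BP_Lever is a lever actor that starts the game's outro when the player reaches it.
; When the player pawn overlaps its sphere, it activates two Niagara effects and snaps the lever mesh to a tilted rotation.
; After a short delay, it finds the BP_CinematicManager in the level and calls PlayOutro on it.
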(event OnComponentBeginOverlap(Sphere)
  (params (OverlappedComponent :type Primitive%20Component%20Object%20Reference) (OtherActor :type Actor%20Object%20Reference) (OtherComp :type Primitive%20Component%20Object%20Reference) (OtherBodyIndex :type Integer) (bFromSweep :type Boolean) (SweepResult :type Hit%20Result%20Structure%20%28by%20ref%29))
  (if (== OtherActor (Game|Player|GetPlayerPawn 0))
    (Components|Activation|Activate (Variables|Default|GetNiagara) true)
    (Transformation|SetRelativeRotation (Variables|Default|Getlever_wall_base_B_blue_lever_wall_B_blue) "0.000000,0.000000,40.000000" false false)
    (Utilities|FlowControl|Delay 1.0)
    (bind _returnvalue (Actor|GetActorOfClass "/Game/CORE/Blueprints/BP_CinematicManager.BP_CinematicManager_C"))
    (Default|PlayOutro _returnvalue)))

(event EventBeginPlay)

(event Collision|EventActorBeginOverlap
  (params (OtherActor :type Actor%20Object%20Reference)))

(event EventTick
  (params (DeltaSeconds :type Float%20%28single-precision%29)))

(fn ConstructionScript)