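; BP_MovingPlat is a moving platform that travels between two points marked by the PosA and PosB components.
; On BeginPlay it maps StartPos from a normalized value to a time on its Timeline, sets the play rate from NewRate and starts playback.
; Each Timeline update lerps the static mesh's world location between both points by the Progress track, without sweeping.
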(event EventBeginPlay
  (Components|Timeline|SetNewTime (Variables|Default|GetTimeline) (Math|Float|MapRangeClamped (Variables|Default|GetStartPos) 0.0 1.0 0.0 (Components|Timeline|GetTimelineLength (Variables|Default|GetTimeline))))
  (Components|Timeline|SetPlayRate (Variables|Default|GetTimeline) (Variables|Default|GetNewRate))
  (bind _progress (Timeline|Timeline Play)
    (:Update
      (Transformation|SetWorldLocation (Variables|Default|GetStaticMesh) (Math|Vector|Lerp(Vector) (Transformation|GetWorldLocation (Variables|Default|GetPosA)) (Transformation|GetWorldLocation (Variables|Default|GetPosB)) _progress) false false))))

(fn ConstructionScript)