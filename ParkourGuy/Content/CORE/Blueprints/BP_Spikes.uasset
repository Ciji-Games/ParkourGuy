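; BP_Spikes is a spiked roller hazard that moves between two points and sends a kill-player message to any actor overlapping its capsule.
; A timeline drives both the roller's position between PosA and PosB and the spin rate of its RotatingMovement component.
; StartPos offsets the timeline's starting time and NewRate sets its play rate, so each instance can have its own phase and speed.
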(event OnComponentBeginOverlap(Capsule)
  (params (OverlappedComponent :type Primitive%20Component%20Object%20Reference) (OtherActor :type Actor%20Object%20Reference) (OtherComp :type Primitive%20Component%20Object%20Reference) (OtherBodyIndex :type Integer) (bFromSweep :type Boolean) (SweepResult :type Hit%20Result%20Structure%20%28by%20ref%29))
  (Class|BPIInteract|Killplayer(Message) OtherActor))

(event EventBeginPlay
  (Components|Movement|SetUpdatedComponent (Variables|Default|GetRotatingMovement) (Variables|Default|GetspikeRoller))
  (Components|Timeline|SetNewTime (Variables|Default|GetTimeline) (Math|Float|MapRangeClamped (Variables|Default|GetStartPos) 0.0 1.0 0.0 (Components|Timeline|GetTimelineLength (Variables|Default|GetTimeline))))
  (Components|Timeline|SetPlayRate (Variables|Default|GetTimeline) (Variables|Default|GetNewRate))
  (bind (_direction _progress _rotationratez) (Timeline|Timeline Play)
    (:Update
      (Variables|/Script/Engine.RotatingMovementComponent|SetRotationRate (Variables|Default|GetRotatingMovement) (Math|Rotator|MakeRotator 0.0 0.0 (Math|Float|Lerp 45.0 5e+02 _rotationratez)))
      (Transformation|SetWorldLocation (Variables|Default|GetspikeRoller) (Math|Vector|Lerp(Vector) (Transformation|GetWorldLocation (Variables|Default|GetPosA)) (Transformation|GetWorldLocation (Variables|Default|GetPosB)) _progress) false false))))

(fn ConstructionScript
  (Components|Movement|SetUpdatedComponent (Variables|Default|GetRotatingMovement) (Variables|Default|GetspikeRoller)))