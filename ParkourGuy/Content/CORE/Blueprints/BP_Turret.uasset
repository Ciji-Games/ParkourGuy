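; Turret that tracks the player and spawns bombs from its barrel while the third-person character is inside its trigger box.
; Box overlap opens or closes a gate on Tick and starts or clears a looping Fire timer set by RateOfFire.
; While open, the mesh eases toward player pawn 0 with RInterpTo, remapping look-at pitch to roll and offsetting yaw to suit its orientation.
; Each Fire call spawns a BP_Bomb at the Barrel socket.
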(event OnComponentBeginOverlap(Box)
  (params (OverlappedComponent :type Primitive%20Component%20Object%20Reference) (OtherActor :type Actor%20Object%20Reference) (OtherComp :type Primitive%20Component%20Object%20Reference) (OtherBodyIndex :type Integer) (bFromSweep :type Boolean) (SweepResult :type Hit%20Result%20Structure%20%28by%20ref%29))
  ;[0.15 0.15 0.15 0.5] Overlap
  (if (Class|GameplayStatics|ObjectIsA OtherActor "/Game/ThirdPerson/Blueprints/BP_ThirdPersonCharacter.BP_ThirdPersonCharacter_C")
    (CallFunction|Open)))

(event OnComponentEndOverlap(Box)
  (params (OverlappedComponent :type Primitive%20Component%20Object%20Reference) (OtherActor :type Actor%20Object%20Reference) (OtherComp :type Primitive%20Component%20Object%20Reference) (OtherBodyIndex :type Integer))
  ;[0.15 0.15 0.15 0.5] Overlap
  (Rendering|Debug|FlushPersistentDebugLines)
  (if (Class|GameplayStatics|ObjectIsA OtherActor "/Game/ThirdPerson/Blueprints/BP_ThirdPersonCharacter.BP_ThirdPersonCharacter_C")
    (CallFunction|Close)))

(event Custom|Close
  (bind _returnvalue (Game|Player|GetPlayerPawn 0))
  (bind _sm_turret_cube (Variables|Default|GetSM_turret_Cube))
  (bind _returnvalue_2 (Transformation|GetWorldLocation _sm_turret_cube))
  (bind _returnvalue_3 (Transformation|GetActorLocation _returnvalue))
  (bind _returnvalue_4 (Math|Rotator|FindLookatRotation _returnvalue_2 _returnvalue_3))
  ;[0.15 0.15 0.15 0.5] Look At tick
  (Utilities|Time|ClearandInvalidateTimerbyHandle (Variables|Default|GetFireLoop))
  (Utilities|FlowControl|Gate true) ; enters at Close
)

(event Custom|Open
  (bind _returnvalue (Game|Player|GetPlayerPawn 0))
  (bind _sm_turret_cube (Variables|Default|GetSM_turret_Cube))
  (bind _returnvalue_2 (Transformation|GetWorldLocation _sm_turret_cube))
  (bind _returnvalue_3 (Transformation|GetActorLocation _returnvalue))
  (bind _returnvalue_4 (Math|Rotator|FindLookatRotation _returnvalue_2 _returnvalue_3))
  ;[0.15 0.15 0.15 0.5] Look At tick
  (bind _returnvalue_5 (Utilities|Time|SetTimerbyFunctionName 0 "Fire" (Variables|Default|GetRateOfFire) true))
  (Variables|Default|SetFireLoop _returnvalue_5)
  (Utilities|FlowControl|Gate true) ; enters at Open
)

(event EventTick
  (params (DeltaSeconds :type Float%20%28single-precision%29))
  (bind _returnvalue (Game|Player|GetPlayerPawn 0))
  (bind _sm_turret_cube (Variables|Default|GetSM_turret_Cube))
  (bind _returnvalue_2 (Transformation|GetWorldLocation _sm_turret_cube))
  (bind _returnvalue_3 (Transformation|GetActorLocation _returnvalue))
  (bind _returnvalue_4 (Math|Rotator|FindLookatRotation _returnvalue_2 _returnvalue_3))
  ;[0.15 0.15 0.15 0.5] Look At tick
  (Utilities|FlowControl|Gate true
    (:Exit
      (Transformation|SetWorldRotation (Variables|Default|GetSM_turret_Cube) (Math|Interpolation|RInterpTo (Transformation|GetWorldRotation (Variables|Default|GetSM_turret_Cube)) (Math|Rotator|MakeRotator (.pitch _returnvalue_4) 0.0 (+ (.yaw _returnvalue_4) 9e+01)) (Utilities|Time|GetWorldDeltaSeconds) (Variables|Default|GetRotaSpeed)) false false))))

(fn ConstructionScript)

(fn Fire
  (Game|SpawnActorfromClass "/Game/CORE/Blueprints/BP_Bomb.BP_Bomb_C" (Math|Transform|MakeTransform (Transformation|GetSocketLocation (Variables|Default|GetSM_turret_Cube) "Barrel") "0, 0, 0" "1.000000,1.000000,1.000000") "Undefined" "MultiplyWithRoot" 0 0))