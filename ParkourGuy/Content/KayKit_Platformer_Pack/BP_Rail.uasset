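; BP_Rail is a spline-driven rail that builds itself from repeated static mesh pieces.
; The construction script divides the spline length by MeshSize and adds a static mesh component at each interval, using the spline's local location and rotation at that distance.
; Pieces are rigid meshes rather than deformed spline meshes, and the event graph holds no runtime logic.
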(event EventBeginPlay)

(event Collision|EventActorBeginOverlap
  (params (OtherActor :type Actor%20Object%20Reference)))

(event EventTick
  (params (DeltaSeconds :type Float%20%28single-precision%29)))

(fn ConstructionScript
  (bind _spline (Variables|Default|GetSpline))
  ;[1 1 1] Create Spline Road
  (for _index (range 0 (Math|Float|Truncate (/ (Spline|GetSplineLength (Variables|Default|GetSpline)) (Variables|Default|GetMeshSize))))
    (AddComponent|AddStaticMeshComponent false (Math|Transform|MakeTransform (Spline|GetLocationatDistanceAlongSpline _spline (* _index (Variables|Default|GetMeshSize)) "Local") (Spline|GetRotationatDistanceAlongSpline _spline (* _index (Variables|Default|GetMeshSize)) "Local") "1.000000,1.000000,1.000000"))))